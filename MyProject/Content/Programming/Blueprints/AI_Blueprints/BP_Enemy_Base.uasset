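; Base enemy Blueprint that feeds player targeting data into its AI controller's Blackboard.
; On BeginPlay it casts the first player character to Player and stores it as TargetActor.
; When an actor tagged Player begins overlapping DetectionRadius, it sets TargetVisible to true; nothing here clears that flag.
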(event `self.ReceiveBeginPlay`
  (`self.SetBlackboardTargetActor`))

(event `self.DetectionRadius.OnComponentBeginOverlap`
  (params (OverlappedComponent :type "PrimitiveComponent Object Reference") (OtherActor :type "Actor Object Reference") (OtherComp :type "PrimitiveComponent Object Reference") (OtherBodyIndex :type Integer) (bFromSweep :type Boolean) (SweepResult :type "HitResult Structure (by ref)"))
  (if (`self.ActorHasTag` OtherActor "Player")
    (`self.SetBlackboardTargetVisible`)))

(fn `SetBlackboardTargetActor`
  (bind _asplayer (cast `/Game/Player` (`GameplayStatics.GetPlayerCharacter` 0)))
  (`BlackboardComponent.SetValueAsObject` (`AIBlueprintHelperLibrary.GetBlackboard` (`AIBlueprintHelperLibrary.GetAIController` self)) "TargetActor" _asplayer))

(fn `SetBlackboardTargetVisible`
  (`BlackboardComponent.SetValueAsBool` (`AIBlueprintHelperLibrary.GetBlackboard` (`AIBlueprintHelperLibrary.GetAIController` self)) "TargetVisible" true)
  (return))

(fn `UserConstructionScript`
  (`parent.UserConstructionScript`))